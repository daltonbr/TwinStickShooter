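; Player hero character for a twin-stick shooter, handling movement, aim-driven firing, and death with respawn.
; Spawns a BP_Weapon onto the mesh's GunSocket at BeginPlay and stores its start transform in BP_TwinStickMode.
; Move axes drive world-space movement; look axes share one path that sets control rotation and pulls the trigger beyond a dead zone, otherwise releasing it.
; AffectHealth updates health; death disables input, then after a delay requests respawn and destroys weapon and character.
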(event `self.ReceiveBeginPlay`
  (bind _mesh (`self.Mesh`))
  (`|ExecutionSequence`
    (:`then_0`
      (bind _returnvalue (`|SpawnActorFromClass` "/Game/Blueprints/BP_Weapon.BP_Weapon_C" (`SceneComponent.K2_GetComponentToWorld` _mesh) "Undefined" "OverrideRootScale" null null))
      (bind _output_get (set `self.Weapon` _returnvalue))
      (`self.K2_AttachToComponent` _output_get _mesh "GunSocket" "SnapToTarget" "KeepRelative" "KeepRelative" true))
    (:`then_1`
      (bind _asbp_twin_stick_mode (cast `/Game/Blueprints/BP_TwinStickMode` (`GameplayStatics.GetGameMode`)))
      (bind _output_get_2 (set `self.GameMode` _asbp_twin_stick_mode))
      (set `/Game/Blueprints/BP_TwinStickMode.PlayerSpawnTransform` (`self.GetTransform`) _output_get_2))))

(event `InputAxis|MoveUp`
  (params (AxisValue :type "Float (single-precision)"))
  ;[1 1 1] Movement
  (`self.AddMovementInput` (1.0 0.0 0.0) AxisValue))

(event `InputAxis|LookUp`
  (params (AxisValue :type "Float (single-precision)"))
  (bind _weapon (`self.Weapon`))
  ;[1 1 1] Rotation
  (bind _returnvalue (`KismetMathLibrary.MakeVector` AxisValue (stale `InputAxis|LookRight` AxisValue)))
  (if (> (`KismetMathLibrary.VSize` _returnvalue) 0.25) :!label _label
    (`Controller.SetControlRotation` (`self.GetController`) (`KismetMathLibrary.MakeRotFromX` _returnvalue))
    (`/Game/Blueprints/BP_Weapon.PullTrigger` _weapon)
    (else
      (`/Game/Blueprints/BP_Weapon.ReleaseTrigger` _weapon))))

(event `InputAxis|LookRight`
  (params (AxisValue :type "Float (single-precision)"))
  ;[1 1 1] Rotation
  (goto _label))

(event `InputAxis|MoveRight`
  (params (AxisValue :type "Float (single-precision)"))
  ;[1 1 1] Movement
  (`self.AddMovementInput` (0.0 1.0 0.0) AxisValue))

(event `self.ReceiveTick`
  (params (DeltaSeconds :type "Float (single-precision)")))

(event `/Game/Blueprints/BPI_IDamageable.AffectHealth`
  (params (Delta :type "Float (single-precision)"))
  (`self.CalculateHealth` Delta)
  (`KismetSystemLibrary.PrintString` (`KismetStringLibrary.Conv_DoubleToString` (`self.Health`)))
  (if (`self.bIsDead`)
    (`self.DisableInput` null)
    (`KismetSystemLibrary.Delay` (`self.DelayBeforeRespawn`))
    (`/Game/Blueprints/BP_TwinStickMode.RespawnPlayer` (`self.GameMode`))
    (`self.K2_DestroyActor` (`self.Weapon`))
    (`self.K2_DestroyActor` self)))

(fn `UserConstructionScript`)